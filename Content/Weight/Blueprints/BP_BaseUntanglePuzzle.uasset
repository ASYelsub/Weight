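; Base untangle puzzle where the player swaps pairs of clicked orbs until no connecting edges overlap, then a completion dispatcher fires.
; At BeginPlay, orb meshes are matched by component creation order to AdjacencyList, which drives spawning of edge meshes stretched between orbs.
; A timeline lerps each swap, re-aligning edges and testing overlaps against "Edge"-tagged components every update.
; Dynamic materials show orb hover, selection and edge crossings.
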(event `self.ReceiveBeginPlay`
  (bind _returnvalue (`self.K2_GetComponentsByClass` "/Script/Engine.StaticMeshComponent"))
  ;[0.05 0.05 0.05] Adds Components to the Array by the order in which they were added to the outliner.
  ; (I.E. Not the order that they appear in the outliner)
  (if (!= (`KismetArrayLibrary.Array_Length` _returnvalue) 0)
    (set `self.StaticMeshComponentsArray` _returnvalue)
    ;[0.05 0.05 0.05] Log Error if Adjacency List does not contain the same amount of elements as the Static Mesh Array.
    (if (== (`KismetArrayLibrary.Array_Length` (`self.AdjacencyList`)) (`KismetArrayLibrary.Array_Length` (`self.StaticMeshComponentsArray`)))
      (`self.SetupSwappableOrbEdges`)
      (else
        (`KismetSystemLibrary.PrintString` (`KismetTextLibrary.Conv_TextToString` (`|FormatText` "{0}'s Adjacency List and Static Mesh Array are not equal length!" (`KismetSystemLibrary.GetDisplayName` self))) true true (struct :`R` 1.0 :`A` 1.0) 10.0)))
    (else
      ;;[0.1 0.1 0.1] Log Error if there are not any Movable Orbs
      (`KismetSystemLibrary.PrintString` (`KismetTextLibrary.Conv_TextToString` (`|FormatText` "{0} has no SwappableOrbs setup!" (`KismetSystemLibrary.GetDisplayName` self))) true true (struct :`R` 1.0 :`A` 1.0) 10.0))))

(event `OnSwappableOrbClicked`
  (params (TouchedComponent :type "PrimitiveComponent Object Reference") (ButtonPressed :type "Key Structure" :default "None"))
  ;[0.05 0.05 0.05] Orb Clicked
  (if (not (`self.IsTimelineRunning`))
    (bind _asstatic_mesh_component (cast `StaticMeshComponent` TouchedComponent))
    ;;[0.1 0.1 0.1] Make sure we are not targeting the selected swappable orb.
    (if (!= _asstatic_mesh_component (`self.SelectedSwappableOrb`))
      (set `self.TargetSwappableOrb` _asstatic_mesh_component)
      (`/Engine/EditorBlueprintResources/StandardMacros.IsValid` (`self.SelectedSwappableOrb`)
        (:`Is Valid`
          (`MeshComponent.SetVectorParameterValueOnMaterials` (`self.TargetSwappableOrb`) "FresnelAlbedo" (`KismetMathLibrary.Conv_LinearColorToVector` (`self.OrbSelectedColour`)))
          (set `self.IsTimelineRunning` true)
          (set `self.OriginalTargetSwappableOrbPosition` (`SceneComponent.K2_GetComponentLocation` (`self.TargetSwappableOrb`)))
          (set `self.OriginalSwappableOrbPosition` (`SceneComponent.K2_GetComponentLocation` (`self.SelectedSwappableOrb`)))
          (bind (_direction _newtrack_0) (`Timeline|Timeline` :!via `PlayFromStart`)
            (:`Update`
              (`SceneComponent.K2_SetWorldLocation` (`self.SelectedSwappableOrb`) (`KismetMathLibrary.VLerp` (`self.OriginalSwappableOrbPosition`) (`self.OriginalTargetSwappableOrbPosition`) _newtrack_0) false false)
              (`SceneComponent.K2_SetWorldLocation` (`self.TargetSwappableOrb`) (`KismetMathLibrary.VLerp` (`self.OriginalTargetSwappableOrbPosition`) (`self.OriginalSwappableOrbPosition`) _newtrack_0) false false)
              (for _array_element (`self.StaticMeshComponentsArray`)
                ;;[0.1 0.1 0.1] Update Edge Look
                (for _array_element_2 (`SceneComponent.GetChildrenComponents` _array_element false)
                  (bind _asstatic_mesh_component_2 (cast `StaticMeshComponent` _array_element_2))
                  (`self.UpdateEdgeLookAtPosition` _asstatic_mesh_component_2)))
              ;;[0.1 0.1 0.1] Update Edge Collision
              (set `self.PuzzleComplete` true)
              (for _array_element_3 (`self.StaticMeshComponentsArray`)
                (for _array_element_4 (`SceneComponent.GetChildrenComponents` _array_element_3 false)
                  (bind _asstatic_mesh_component_3 (cast `StaticMeshComponent` _array_element_4))
                  (bind _collided (`self.UpdateEdgeCollisionColour` _asstatic_mesh_component_3))
                  (if _collided
                    (set `self.PuzzleComplete` false)))))
            (:`Finished`
              ;;[0.1 0.1 0.1] Reset everything. Check for win condition.
              (`MeshComponent.SetVectorParameterValueOnMaterials` (`self.TargetSwappableOrb`) "FresnelAlbedo" (`KismetMathLibrary.Conv_LinearColorToVector` (`self.OrbUnselectedColour`)))
              (`MeshComponent.SetVectorParameterValueOnMaterials` (`self.SelectedSwappableOrb`) "FresnelAlbedo" (`KismetMathLibrary.Conv_LinearColorToVector` (`self.OrbUnselectedColour`)))
              (set `self.TargetSwappableOrb` null)
              (set `self.SelectedSwappableOrb` null)
              (set `self.IsTimelineRunning` false)
              (if (`self.PuzzleComplete`)
                (`self.PuzzleCompleteDispatcher`)))))
        (:`Is Not Valid`
          (set `self.SelectedSwappableOrb` _asstatic_mesh_component)
          (`MeshComponent.SetVectorParameterValueOnMaterials` (`self.TargetSwappableOrb`) "FresnelAlbedo" (`KismetMathLibrary.Conv_LinearColorToVector` (`self.OrbSelectedColour`))))))))

(event `OnSwappableOrbMouseEnter`
  (params (TouchedComponent :type "PrimitiveComponent Object Reference"))
  ;[0.05 0.05 0.05] Orb Mouse Enter
  (bind _asstatic_mesh_component (cast `StaticMeshComponent` TouchedComponent))
  (if (and (!= _asstatic_mesh_component (`self.TargetSwappableOrb`)) (!= _asstatic_mesh_component (`self.SelectedSwappableOrb`)))
    (`MeshComponent.SetVectorParameterValueOnMaterials` _asstatic_mesh_component "FresnelAlbedo" (`KismetMathLibrary.Conv_LinearColorToVector` (`self.OrbMouseOverColour`)))))

(event `OnSwappableOrbMouseExit`
  (params (TouchedComponent :type "PrimitiveComponent Object Reference"))
  ;[0.05 0.05 0.05] Orb Mouse Over
  (bind _asstatic_mesh_component (cast `StaticMeshComponent` TouchedComponent))
  (if (and (!= _asstatic_mesh_component (`self.TargetSwappableOrb`)) (!= _asstatic_mesh_component (`self.SelectedSwappableOrb`)))
    (`MeshComponent.SetVectorParameterValueOnMaterials` _asstatic_mesh_component "FresnelAlbedo" (`KismetMathLibrary.Conv_LinearColorToVector` (`self.OrbUnselectedColour`)))))

(fn `SetupSwappableOrbEdges`
  (locals (SwappableOrb :type "StaticMeshComponent Object Reference") (SwappableOrbConnection :type "StaticMeshComponent Object Reference") (`New Edge` :type "StaticMeshComponent Object Reference") (SwappableOrbIndex :type Integer))
  (bind _nodediameter (`self.NodeDiameter`))
  ;[0.05 0.05 0.05] Loop through all SwappableOrbs
  (for (_array_element _array_index) (`self.StaticMeshComponentsArray`)
    (set `local.SwappableOrb` _array_element)
    (set `local.SwappableOrbIndex` _array_index)
    ;[0.05 0.05 0.05] Set Dynamic Material for Orb
    (bind _returnvalue (`KismetMaterialLibrary.CreateDynamicMaterialInstance` "/Game/Weight/Materials/M_OrbNode.M_OrbNode"))
    (`PrimitiveComponent.SetMaterial` (`local.SwappableOrb`) 0 _returnvalue)
    ;[0.05 0.05 0.05] Set Swappable Orb Diameter
    (`SceneComponent.SetWorldScale3D` (`local.SwappableOrb`) (`KismetMathLibrary.MakeVector` _nodediameter _nodediameter _nodediameter))
    ;[0.05 0.05 0.05] Bind to SwappableOrb cursor enter
    (add `PrimitiveComponent.OnBeginCursorOver` (`local.SwappableOrb`) (`|CreateDelegate` :!event `OnSwappableOrbMouseEnter`))
    ;[0.05 0.05 0.05] Bind to SwappableOrb cursor exit
    (add `PrimitiveComponent.OnEndCursorOver` (`local.SwappableOrb`) (`|CreateDelegate` :!event `OnSwappableOrbMouseExit`))
    ;[0.05 0.05 0.05] Bind to SwappableOrb click event.
    (add `PrimitiveComponent.OnClicked` (`local.SwappableOrb`) (`|CreateDelegate` :!event `OnSwappableOrbClicked`))
    ;[0.05 0.05 0.05] Loop through Adjacency List
    (for _array_element_2 (`.UnorderedIntegerArray_6_82CC1C3F4846CED28452B98CFF5BB973` (break `/Game/Weight/Blueprints/F_UnorderedIntegerArray` (`|GetArrayItem` (`self.AdjacencyList`) (`local.SwappableOrbIndex`))))
      ;[0.05 0.05 0.05] Create and attach the edge to the origin node.
      (set `local.SwappableOrbConnection` (`|GetArrayItem` (`self.StaticMeshComponentsArray`) _array_element_2))
      (bind _returnvalue_2 (`AddComponent|NODE_AddStaticMeshComponent-0` :`bManualAttachment` true))
      (bind _output_get (set `local.New Edge` _returnvalue_2))
      (`SceneComponent.K2_AttachToComponent` _output_get (`local.SwappableOrb`) "None" "KeepWorld" "KeepRelative" "KeepWorld" false)
      ;[0.05 0.05 0.05] Set Dynamic Material for Edge
      (bind _returnvalue_3 (`KismetMaterialLibrary.CreateDynamicMaterialInstance` "/Game/Weight/Materials/M_OrbEdge.M_OrbEdge"))
      (`PrimitiveComponent.SetMaterial` (`local.New Edge`) 0 _returnvalue_3)
      ;[0.05 0.05 0.05] Generate Edge Data For Future
      (`BlueprintMapLibrary.Map_Add` (`self.EdgesData`) (`local.New Edge`) (make `/Game/Weight/Blueprints/F_EdgeData` (`local.SwappableOrb`) (`local.SwappableOrbConnection`)))
      ;[0.05 0.05 0.05] Orient the cylinder.
      (`self.UpdateEdgeLookAtPosition` (`local.New Edge`)))
    ;[0.05 0.05 0.05] Update Edge Collision
    (for _array_element_3 (`self.StaticMeshComponentsArray`)
      (for _array_element_4 (`SceneComponent.GetChildrenComponents` _array_element_3 false)
        (bind _asstatic_mesh_component (cast `StaticMeshComponent` _array_element_4))
        (`self.UpdateEdgeCollisionColour` _asstatic_mesh_component)))))

(fn `UpdateEdgeCollisionColour`
  (params (Edge :type "StaticMeshComponent Object Reference"))
  (returns (Collided :type Boolean))
  (locals (TargetEdge :type "StaticMeshComponent Object Reference"))
  (bind _output_get (set `local.TargetEdge` Edge))
  ;[0.05 0.05 0.05] Check collided components, change colour based on result.
  (for _array_element (`PrimitiveComponent.GetOverlappingComponents` _output_get)
    (if (and (`ActorComponent.ComponentHasTag` _array_element "Edge") (`PrimitiveComponent.IsOverlappingComponent` (`local.TargetEdge`) _array_element))
      (`MeshComponent.SetVectorParameterValueOnMaterials` (`local.TargetEdge`) "Colour" (1.0 0.0 0.0))
      (return true)
      (else
        (`MeshComponent.SetVectorParameterValueOnMaterials` (`local.TargetEdge`) "Colour" (0.0 1.0 0.0)))))
  (return false))

(fn `UpdateEdgeLookAtPosition`
  (params (Edge :type "StaticMeshComponent Object Reference"))
  (locals (TargetEdge :type "StaticMeshComponent Object Reference") (SelectedSwappableOrb :type "StaticMeshComponent Object Reference") (TargetSwappableOrb :type "StaticMeshComponent Object Reference"))
  (bind _edgediameter (`self.EdgeDiameter`))
  (bind (_startswappableorb _endswappableorb) (break `/Game/Weight/Blueprints/F_EdgeData` (`BlueprintMapLibrary.Map_Find` (`self.EdgesData`) Edge)))
  ;[0.05 0.05 0.05] Setup local variables.
  (set `local.TargetEdge` Edge)
  (set `local.SelectedSwappableOrb` _startswappableorb)
  (set `local.TargetSwappableOrb` _endswappableorb)
  ;[0.05 0.05 0.05] Set the position of the Cylinder between the two swappable orbs.
  (`SceneComponent.K2_SetWorldLocation` (`local.TargetEdge`) (/ (+ (`SceneComponent.K2_GetComponentLocation` (`local.TargetSwappableOrb`)) (`SceneComponent.K2_GetComponentLocation` (`local.SelectedSwappableOrb`))) (2.0 2.0 2.0)) false false)
  ;[0.05 0.05 0.05] Set the rotation of the Cylinder
  (`SceneComponent.K2_SetWorldRotation` (`local.TargetEdge`) (`KismetMathLibrary.FindLookAtRotation` (`SceneComponent.K2_GetComponentLocation` (`local.SelectedSwappableOrb`)) (`SceneComponent.K2_GetComponentLocation` (`local.TargetSwappableOrb`))) false false)
  ;[0.05 0.05 0.05] Scale the Cylinder along its forward axis until it touches both swappable orbs.
  (`SceneComponent.SetWorldScale3D` (`local.TargetEdge`) (`KismetMathLibrary.MakeVector` (`KismetMathLibrary.SafeDivide` (- (`KismetMathLibrary.Vector_Distance` (`SceneComponent.K2_GetComponentLocation` (`local.TargetSwappableOrb`)) (`SceneComponent.K2_GetComponentLocation` (`local.SelectedSwappableOrb`))) 10.0) 100.0) _edgediameter _edgediameter)))

(fn `UserConstructionScript`
  (locals (SwappableOrb :type "StaticMeshComponent Object Reference") (SwappableOrbConnection :type "StaticMeshComponent Object Reference") (SplineMesh :type "SplineMeshComponent Object Reference")))